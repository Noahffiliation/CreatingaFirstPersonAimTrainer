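; Target spawner that runs a single ten-second aim-trainer round and records the best score.
; StartSpawning fires once, spawns an initial batch of BP_Targets, then adds more on a looping timer up to a population cap.
; Targets appear at random points in an editable box, rotated toward the player camera with a yaw offset.
; At round end it destroys all targets and saves MatchScore, accumulated through UpdateMatchScore, to GI_AimTrainer if higher.
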(event `UpdateMatchScore`
  (params (Points :type Integer))
  (bind _output_get (set `self.MatchScore` (+ Points (`self.MatchScore`))))
  (`KismetSystemLibrary.PrintString` (`KismetStringLibrary.Conv_IntToString` _output_get)))

(event `self.ReceiveBeginPlay`
  (bind _asgi_aim_trainer (cast `/Game/Blueprints/FirstPersonTemplate/GI_AimTrainer` (`GameplayStatics.GetGameInstance`))))

(event `StartSpawning`
  (bind _matchscore (`self.MatchScore`))
  (`/Engine/EditorBlueprintResources/StandardMacros.DoOnce` false
    (:`Completed`
      (bind _returnvalue (`KismetSystemLibrary.K2_SetTimerDelegate` (delegate `SpawnTarget`) 1.0 true))
      (set `self.TargetSpawner` _returnvalue)
      (for _ (range 9)
        (`self.SpawnTarget`))
      (`KismetSystemLibrary.Delay` 10.0)
      (`KismetSystemLibrary.K2_ClearAndInvalidateTimerHandle` (`self.TargetSpawner`))
      (bind _outactors (`GameplayStatics.GetAllActorsOfClass` "/Game/Blueprints/Target/BP_Target.BP_Target_C"))
      (for _array_element _outactors
        (`self.K2_DestroyActor` _array_element))
      (bind _asgi_aim_trainer (cast `/Game/Blueprints/FirstPersonTemplate/GI_AimTrainer` (`GameplayStatics.GetGameInstance`)))
      (if (> _matchscore (`/Game/Blueprints/FirstPersonTemplate/GI_AimTrainer.Score` _asgi_aim_trainer))
        (set `/Game/Blueprints/FirstPersonTemplate/GI_AimTrainer.Score` _matchscore _asgi_aim_trainer)))))

(event `SpawnTarget`
  (bind _spawn_area (`self.Spawn_Area`))
  (bind _outactors (`GameplayStatics.GetAllActorsOfClass` "/Game/Blueprints/Target/BP_Target.BP_Target_C"))
  (if (<= (`KismetArrayLibrary.Array_Length` _outactors) 10)
    (bind _output_get (set `self.SpawnLocation` (`KismetMathLibrary.RandomPointInBoundingBox` (`SceneComponent.K2_GetComponentLocation` _spawn_area) (`BoxComponent.GetScaledBoxExtent` _spawn_area))))
    (bind (_returnvalue_roll _returnvalue_pitch _returnvalue_yaw) (`KismetMathLibrary.BreakRotator` (`KismetMathLibrary.FindLookAtRotation` _output_get (`SceneComponent.K2_GetComponentLocation` (`PlayerCameraManager.TransformComponent` (`GameplayStatics.GetPlayerCameraManager` 0))))))
    (`|SpawnActorFromClass` "/Game/Blueprints/Target/BP_Target.BP_Target_C" (`KismetMathLibrary.MakeTransform` _output_get (`KismetMathLibrary.MakeRotator` _returnvalue_roll _returnvalue_pitch (- _returnvalue_yaw 90.0))) "Undefined" "OverrideRootScale" null null)))

(fn `UserConstructionScript`
  (`BoxComponent.SetBoxExtent` (`self.Spawn_Area`) (`self.Box Extent`) true))